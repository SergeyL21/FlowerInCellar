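; BP_Bottle is an interactable bottle actor with a text label that turns to face the player.
; Every Tick rotates the TextRender toward player character 0 with a look-at rotation, and the zero interp speed on RInterpTo makes it snap instantly.
; It overrides GetInteractableType to return its Type variable without calling the parent, while the construction script only runs the parent's.
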(event `self.ReceiveTick`
  (params (DeltaSeconds :type "Float (single-precision)"))
  (bind _textrender (`self.TextRender`))
  (`SceneComponent.K2_SetWorldRotation` _textrender (`KismetMathLibrary.RInterpTo` (`SceneComponent.K2_GetComponentRotation` _textrender) (`KismetMathLibrary.FindLookAtRotation` (`SceneComponent.K2_GetComponentLocation` _textrender) (`self.K2_GetActorLocation` (`GameplayStatics.GetPlayerCharacter` 0))) DeltaSeconds 0.0) false false))

(fn `GetInteractableType`
  (returns (ActorType :type "/Game/Blueprints/EInteractableType Enum"))
  (locals (Type :type "/Game/Blueprints/EInteractableType Enum" :default "NewEnumerator1"))
  (return (`local.Type`)))

(fn `UserConstructionScript`
  (`parent.UserConstructionScript`))